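; Player-controllable tank Blueprint that handles camera aiming and firing.
; On BeginPlay it assigns the turret and barrel meshes, then passes those components to SetTurretReference and SetBarrelReference.
; Aim axes drive a split camera rig, yawing the azimuth gimbal and pitching the spring arm separately, while the fire action calls Fire.
; Turret and barrel movement and projectile logic are not implemented in these graphs.
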(event `self.ReceiveBeginPlay`
  (bind _turret (`self.Turret`))
  (bind _barrel (`self.Barrel`))
  (`|ExecutionSequence`
    (:`then_0`
      (`StaticMeshComponent.SetStaticMesh` _turret "/Game/Improved_Tank/tank_fbx_Turret.tank_fbx_Turret")
      (`self.SetTurretReference` _turret))
    (:`then_1`
      (`StaticMeshComponent.SetStaticMesh` _barrel "/Game/Improved_Tank/tank_fbx_Barrel.tank_fbx_Barrel")
      (`self.SetBarrelReference` _barrel))))

(event `InputAxis|AimAzimuth`
  (params (AxisValue :type "Float (single-precision)"))
  ;[1 1 1] Camera Input Binding
  (`SceneComponent.K2_AddLocalRotation` (`self.Azimuth Gimbal`) (`KismetMathLibrary.MakeRotator` 0.0 0.0 AxisValue) false false))

(event `InputAxis|AimElevation`
  (params (AxisValue :type "Float (single-precision)"))
  ;[1 1 1] Camera Input Binding
  (`SceneComponent.K2_AddLocalRotation` (`self.SpringArm`) (`KismetMathLibrary.MakeRotator` 0.0 AxisValue) false false))

(event `InputAction|FireProjectile`
  (params (Key :type "Key Structure"))
  ;[1 1 1] Fire projectile
  (:`Pressed`
    (`self.Fire`)))

(fn `UserConstructionScript`)